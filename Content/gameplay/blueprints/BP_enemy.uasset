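; Zombie enemy character whose sight and hit events feed blackboard flags on its AI controller.
; Seeing the player through PawnSensing sets a seen flag; GetHit raises an attacked flag for a few seconds, plays a hit montage and runs a timeline-driven dodge-back nudge.
; AttackPlayer sphere-traces ahead and plays the attack montage on finding the player, applying no damage.
; Older direct chase logic remains unconnected.
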(event OnSeePawn(PawnSensing)
  (params (Pawn :type Pawn%20Object%20Reference))
  (Utilities|Casting|CastToBP_ThirdPersonCharacter Pawn)
  (AI|Components|Blackboard|SetValueasBool (AI|GetBlackboard (AI|GetAIController self)) (Utilities|Name|MakeLiteralName "hasSeenPlayer?") true))

(event Custom|AttackPlayer
  (bind _returnvalue (Transformation|GetActorLocation))
  (bind (_outhit _returnvalue_2) (Collision|SphereTraceForObjects _returnvalue (+ _returnvalue (* (Math|Vector|GetForwardVector (Transformation|GetActorRotation)) 2.5e+02)) 1.2e+02 (Utilities|Array|MakeArray "ObjectTypeQuery3") false 0 "None"))
  (if _returnvalue_2
    (Utilities|Casting|CastToBP_ThirdPersonCharacter (.HitActor (Collision|BreakHitResult _outhit)))
    (Development|PrintString "attackplayer")
    (Animation|PlayAnimMontage "/Game/gameplay/gzombie_Attack_Montage.gzombie_Attack_Montage" 1.0 "None")))

(event Custom|GetHit
  (AI|Components|Blackboard|SetValueasBool (AI|GetBlackboard (AI|GetAIController self)) (Utilities|Name|MakeLiteralName "beingAttaked?") true)
  (Animation|PlayAnimMontage "/Game/gameplay/gzombie_hitback_Montage.gzombie_hitback_Montage" 1.0 "None")
  (CallFunction|Dodgeback)
  (Utilities|FlowControl|Delay 5.0)
  (AI|Components|Blackboard|SetValueasBool (AI|GetBlackboard (AI|GetAIController self)) (Utilities|Name|MakeLiteralName "beingAttaked?") false)
  (Components|Activation|Activate (Variables|Character|GetCharacterMovement) false))

(event Custom|Dodgeback
  (Animation|PlayAnimMontage 0 1.0 "None")
  (bind _新建轨道_0 (Timeline|时间轴 PlayFromStart)
    (:Update
      (Transformation|SetActorLocation (Math|Vector|Lerp(Vector) (Transformation|GetActorLocation) (+ (Transformation|GetActorLocation) (* (Math|Vector|GetRightVector (Variables|Character|GetMesh)) -5.0)) _新建轨道_0) false false))))

(event EventBeginPlay)

(event Collision|EventActorBeginOverlap
  (params (OtherActor :type Actor%20Object%20Reference)))

(event EventTick
  (params (DeltaSeconds :type Float%20%28single-precision%29)))

(fn ConstructionScript)