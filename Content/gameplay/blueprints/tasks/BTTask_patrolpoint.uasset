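; Behavior tree task that makes an AI pawn patrol the actors in the PatrolPath map of its AIPathComponent.
; It moves to the current actor, waits on a timer, then advances the index, wrapping to the start.
; The wait time comes from the map value of the first key, whichever point is reached.
; The task loops without ever finishing successfully, failing only on a missing component, empty path or failed move.
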(event Custom|MoveToPatrolPoint
  (bind _patrol_path (Variables|Default|GetPatrol%20Path))
  (bind _keys (Utilities|Map|Keys (Variables|Default|GetPatrol%20Path)))
  (AI|AIMoveTo (stale EventReceiveExecuteAI ControlledPawn) (Transformation|GetActorLocation (Utilities|Array|Get(acopy) _keys (Variables|Default|GetCurrentPatrolPath))) 0 5.0 false
    (:OnSuccess
      (bind _keys_2 (Utilities|Map|Keys _patrol_path))
      (Utilities|Time|SetTimerbyEvent (EventDispatchers|CreateEvent :!event Custom|OnEndWaiting) (.Value (Utilities|Map|Find _patrol_path (Utilities|Array|Get(acopy) _keys_2)))))
    (:OnFail
      (AI|BehaviorTree|FinishExecute false))))

(event Custom|OnEndWaiting
  (bind _result (Math|Integer|IncrementInt (Variables|Default|GetCurrentPatrolPath))
    (:%20%20
      (if (>= _result (Utilities|Map|Length (Variables|Default|GetPatrol%20Path)))
        (Variables|Default|SetCurrentPatrolPath 0)
        (CallFunction|MovetoPatrolPoint)
        (else
          (CallFunction|MovetoPatrolPoint))))))

(event EventReceiveExecuteAI
  (params (OwnerController :type AI%20Controller%20Object%20Reference) (ControlledPawn :type Pawn%20Object%20Reference))
  (bind _returnvalue (Actor|GetComponentbyClass ControlledPawn "/Game/gameplay/blueprints/AIPathComponent.AIPathComponent_C"))
  (bind _patrolpath (Variables|/Game/gameplay/blueprints/AIPathComponent.AIPathComponent_C|GetPatrolPath _returnvalue))
  (Utilities|IsValid _returnvalue
    (:Is%20Valid
      (if (> (Utilities|Map|Length _patrolpath) 0)
        (Variables|Default|SetPatrol%20Path _patrolpath)
        (CallFunction|MovetoPatrolPoint)
        (else
          (AI|BehaviorTree|FinishExecute false))))
    (:Is%20Not%20Valid
      (AI|BehaviorTree|FinishExecute false))))